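; BP_Projectile is a short-lived projectile actor that scores kills for the player and expires after a fixed lifespan.
; Its sphere overlap destroys it on contact with a BP_Player or BP_Tunnel.
; On hitting a BP_Enemy, if its instigator is a BP_Player, it adds score to that player, prints it, and destroys both enemy and projectile; otherwise it only logs a debug message.
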(event `self.ReceiveBeginPlay`
  (`self.SetLifeSpan` 10.0))

(event `self.Sphere.OnComponentBeginOverlap`
  (params (OverlappedComponent :type "PrimitiveComponent Object Reference") (OtherActor :type "Actor Object Reference") (OtherComp :type "PrimitiveComponent Object Reference") (OtherBodyIndex :type Integer) (bFromSweep :type Boolean) (SweepResult :type "HitResult Structure (by ref)"))
  (cast `/Game/InfiniteMatrix/Blueprints/BP_Player` OtherActor
    (:`then`
      (`self.K2_DestroyActor` :!label _label))
    (:`CastFailed`
      (cast `/Game/InfiniteMatrix/Blueprints/BP_Tunnel` OtherActor
        (:`then`
          (goto _label))
        (:`CastFailed`
          (cast `/Game/InfiniteMatrix/Blueprints/BP_Enemy` OtherActor)
          (bind _asbp_player (cast `/Game/InfiniteMatrix/Blueprints/BP_Player` (`self.GetInstigator`))
            (:`then`
              (bind _output_get (set `/Game/InfiniteMatrix/Blueprints/BP_Player.Score` (+ (`/Game/InfiniteMatrix/Blueprints/BP_Player.Score` _asbp_player) 10) _asbp_player))
              (`KismetSystemLibrary.PrintString` (`KismetStringLibrary.Conv_IntToString` _output_get))
              (`self.K2_DestroyActor` OtherActor)
              (goto _label))
            (:`CastFailed`
              (`KismetSystemLibrary.PrintString` "Not palyer"))))))))

(fn `UserConstructionScript`)